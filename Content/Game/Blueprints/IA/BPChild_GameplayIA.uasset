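; AI character Blueprint for a person screened at BP_ValidationGate, carrying either a suitcase or a backpack.
; BeginPlay makes a weighted random pick from DT_InfoIA for suspicion traits and name pools; ReActivate rerolls using the cached total weight.
; DropBelonging hides the carried bag and hands it to the gate, while RotateActor turns the character around via timeline.
; It also tracks Look-volume overlaps and prints its profile every tick for debugging.
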(event OnComponentBeginOverlap(Look)
  (params (OverlappedComponent :type Primitive%20Component%20Object%20Reference) (OtherActor :type Actor%20Object%20Reference) (OtherComp :type Primitive%20Component%20Object%20Reference) (OtherBodyIndex :type Integer) (bFromSweep :type Boolean) (SweepResult :type Hit%20Result%20Structure%20%28by%20ref%29))
  (Variables|Default|SetbPlayer%20IN true))

(event OnComponentEndOverlap(Look)
  (params (OverlappedComponent :type Primitive%20Component%20Object%20Reference) (OtherActor :type Actor%20Object%20Reference) (OtherComp :type Primitive%20Component%20Object%20Reference) (OtherBodyIndex :type Integer))
  (Variables|Default|SetbPlayer%20IN false))

(event Custom|RotateActor
  (Variables|Default|SetActorRotation (Transformation|GetActorRotation))
  (bind _rotatetime (Timeline|Timeline PlayFromStart)
    (:Update
      (Transformation|SetActorRotation (Math|Rotator|Lerp(Rotator) (Variables|Default|GetActorRotation) (Math|Rotator|MakeRotator (.Roll (Math|Rotator|BreakRotator (Variables|Default|GetActorRotation))) (.Pitch (Math|Rotator|BreakRotator (Variables|Default|GetActorRotation))) (+ (.Yaw (Math|Rotator|BreakRotator (Variables|Default|GetActorRotation))) 1.8e+02)) _rotatetime true)))))

(event Custom|ReActivate
  ;[0.15 0.15 0.15 0.5] Ai Data
  (Variables|Default|SetRandomValue (Math|Random|RandomFloatinRange 0.0 (Variables|Default|GetTotalWeight)))
  (Variables|Default|SetActualSum 0.0)
  (bind _array_element (Utilities|Array|ForEachLoopwithBreak (Variables|Default|GetInfoIARowName) :!label _label)
    (:LoopBody
      (bind _returnvalue (Utilities|GetDataTableRow "/Game/Game/Blueprints/IA/AI_Data/DT_InfoIA.DT_InfoIA" _array_element)
        (:then
          (Variables|Default|SetActualSum (+ (.Probability (Utilities|Struct|BreakS_InfoIA _returnvalue)) (Variables|Default|GetActualSum)))
          (if (<= (Variables|Default|GetRandomValue) (Variables|Default|GetActualSum))
            (Variables|Default|SetSelectedRowName _array_element)
            (goto _label Break)))))
    (:Completed
      (Variables|Default|SetLoopCompleted true)
      (bind _returnvalue_2 (Utilities|GetDataTableRow "/Game/Game/Blueprints/IA/AI_Data/DT_InfoIA.DT_InfoIA" (Variables|Default|GetSelectedRowName))
        (:then
          (Variables|Temp|SetSuspisious%20Items (.SuspisiousItems (Utilities|Struct|BreakS_InfoIA _returnvalue_2)))
          (Variables|Temp|SetMetalic%20Item (.MetalicItem (Utilities|Struct|BreakS_InfoIA _returnvalue_2)))
          (Variables|Temp|SetStrange%20Behavior (.StrangeBehavior (Utilities|Struct|BreakS_InfoIA _returnvalue_2)))
          (Variables|Temp|SetFake%20ID (.FakeID (Utilities|Struct|BreakS_InfoIA _returnvalue_2)))
          (Variables|Default|SetIA%20Name (Utilities|String|StringToName (Utilities|String|EnumtoString (Utilities|Array|Get(acopy) (.Possiblename (Utilities|Struct|BreakS_InfoIA _returnvalue_2)) (Math|Random|RandomIntegerinRange 0 (Utilities|Array|Length (.Possiblename (Utilities|Struct|BreakS_InfoIA _returnvalue_2))))))))
          (Variables|Default|SetIA%20Surname (Utilities|String|StringToName (Utilities|String|EnumtoString (Utilities|Array|Get(acopy) (.PossibleSurname (Utilities|Struct|BreakS_InfoIA _returnvalue_2)) (Math|Random|RandomIntegerinRange 0 (Utilities|Array|Length (.PossibleSurname (Utilities|Struct|BreakS_InfoIA _returnvalue_2))))))))
          (Variables|Default|SetbBelonging (Math|Random|RandomBool))
          (Rendering|SetVisibility (Variables|Default|GetSuitcase) (select (Variables|Default|GetbBelonging) true false) false)
          (Rendering|SetVisibility (Variables|Default|GetBackpack) (select (Variables|Default|GetbBelonging) false true) false)
          (bind _returnvalue_3 (Actor|GetActorOfClass "/Game/Game/Blueprints/ValidationGate/BP_ValidationGate.BP_ValidationGate_C"))
          (Variables|Default|SetGate%20REF _returnvalue_3))))))

(event Custom|Drop%20Belonging
  (bind _bbelonging (Variables|Default|GetbBelonging))
  (bind _suitcase (Variables|Default|GetSuitcase))
  (bind _backpack (Variables|Default|GetBackpack))
  (bind _returnvalue (select _bbelonging _suitcase _backpack))
  (Variables|Default|SetTransform%20Beloging (Transformation|GetRelativeTransform _returnvalue))
  (Rendering|SetVisibility _returnvalue false false)
  (Default|MoveBelonging (Variables|Default|GetGate%20REF) (Variables|Default|GetbBelonging) (Variables|Temp|GetSuspisious%20Items)))

(event EventBeginPlay
  ;[0.15 0.15 0.15 0.5] Ai Data
  (Variables|Default|SetLoopCompleted false)
  (Variables|Default|SetTotalWeight 0.0)
  (bind _outrownames (DataTable|GetDataTableRowNames "/Game/Game/Blueprints/IA/AI_Data/DT_InfoIA.DT_InfoIA"))
  (bind _output_get (Variables|Default|SetInfoIARowName _outrownames))
  (for _array_element _output_get
    (bind _returnvalue (Utilities|GetDataTableRow "/Game/Game/Blueprints/IA/AI_Data/DT_InfoIA.DT_InfoIA" _array_element)
      (:then
        (Variables|Default|SetTotalWeight (+ (.Probability (Utilities|Struct|BreakS_InfoIA _returnvalue)) (Variables|Default|GetTotalWeight))))))
  (Variables|Default|SetRandomValue (Math|Random|RandomFloatinRange 0.0 (Variables|Default|GetTotalWeight)))
  (Variables|Default|SetActualSum 0.0)
  (bind _array_element_2 (Utilities|Array|ForEachLoopwithBreak (Variables|Default|GetInfoIARowName) :!label _label)
    (:LoopBody
      (bind _returnvalue_2 (Utilities|GetDataTableRow "/Game/Game/Blueprints/IA/AI_Data/DT_InfoIA.DT_InfoIA" _array_element_2)
        (:then
          (Variables|Default|SetActualSum (+ (.Probability (Utilities|Struct|BreakS_InfoIA _returnvalue_2)) (Variables|Default|GetActualSum)))
          (if (<= (Variables|Default|GetRandomValue) (Variables|Default|GetActualSum))
            (Variables|Default|SetSelectedRowName _array_element_2)
            (goto _label Break)))))
    (:Completed
      (Variables|Default|SetLoopCompleted true)
      (bind _returnvalue_3 (Utilities|GetDataTableRow "/Game/Game/Blueprints/IA/AI_Data/DT_InfoIA.DT_InfoIA" (Variables|Default|GetSelectedRowName))
        (:then
          (Variables|Temp|SetSuspisious%20Items (.SuspisiousItems (Utilities|Struct|BreakS_InfoIA _returnvalue_3)))
          (Variables|Temp|SetMetalic%20Item (.MetalicItem (Utilities|Struct|BreakS_InfoIA _returnvalue_3)))
          (Variables|Temp|SetStrange%20Behavior (.StrangeBehavior (Utilities|Struct|BreakS_InfoIA _returnvalue_3)))
          (Variables|Temp|SetFake%20ID (.FakeID (Utilities|Struct|BreakS_InfoIA _returnvalue_3)))
          (Variables|Default|SetIA%20Name (Utilities|String|StringToName (Utilities|String|EnumtoString (Utilities|Array|Get(acopy) (.Possiblename (Utilities|Struct|BreakS_InfoIA _returnvalue_3)) (Math|Random|RandomIntegerinRange 0 (Utilities|Array|Length (.Possiblename (Utilities|Struct|BreakS_InfoIA _returnvalue_3))))))))
          (Variables|Default|SetIA%20Surname (Utilities|String|StringToName (Utilities|String|EnumtoString (Utilities|Array|Get(acopy) (.PossibleSurname (Utilities|Struct|BreakS_InfoIA _returnvalue_3)) (Math|Random|RandomIntegerinRange 0 (Utilities|Array|Length (.PossibleSurname (Utilities|Struct|BreakS_InfoIA _returnvalue_3))))))))
          (Variables|Default|SetbBelonging (Math|Random|RandomBool))
          (Rendering|SetVisibility (Variables|Default|GetSuitcase) (select (Variables|Default|GetbBelonging) true false) false)
          (Rendering|SetVisibility (Variables|Default|GetBackpack) (select (Variables|Default|GetbBelonging) false true) false)
          (bind _returnvalue_4 (Actor|GetActorOfClass "/Game/Game/Blueprints/ValidationGate/BP_ValidationGate.BP_ValidationGate_C"))
          (Variables|Default|SetGate%20REF _returnvalue_4))))))

(event EventTick
  (params (DeltaSeconds :type Float%20%28single-precision%29))
  (Utilities|FlowControl|Sequence
    (:then_0
      ;[0.15 0.15 0.15 0.5] Print IA Info
      (if (Variables|Default|GetLoopCompleted)
        (Development|PrintString (Utilities|String|Append "Name :" (Utilities|String|ToString(Name) (Variables|Default|GetIA%20Name)) " 
Surname :" (Utilities|String|ToString(Name) (Variables|Default|GetIA%20Surname)) " 
Suspisious Items :" (Utilities|String|ToString(Boolean) (Variables|Temp|GetSuspisious%20Items)) " 
Metalic Item :" (Utilities|String|ToString(Boolean) (Variables|Temp|GetMetalic%20Item)) " 
Strange Behavior :" (Utilities|String|ToString(Boolean) (Variables|Temp|GetStrange%20Behavior)) " 
Fake ID :" (Utilities|String|ToString(Boolean) (Variables|Temp|GetFake%20ID)) (Utilities|String|Append " 
Velocity :" (Utilities|String|ToString(Vector) (Transformation|GetVelocity)))) true false "(R=1.000000,G=0.000000,B=0.000000,A=1.000000)" 0.0)))))

(fn ConstructionScript
  (|CallParentFunction))