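; Manager that spawns AI passengers and directs the first through a security-gate routine.
; Construction script sizes the spawn-location array to the AI count; BeginPlay spawns them only if no location is zero.
; OrderIA steps an enum-driven AIMoveTo sequence from bag drop through gate to pickup, with long triggers diverting to a check zone at later stages.
; After pickup, the passenger walks out, then teleports to spawn and reactivates for another loop.
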(event Custom|SpawnIA
  ;[0.15 0.15 0.15 0.5] Spawn selected number of IA
  (for _array_element (Variables|LocationPoint|GetSpawnLocation%20IA)
    (if (Class|KismetMathLibrary|EqualExactlyVectorVector _array_element "0, 0, 0")
      (Math|Integer|IncrementInt (Variables|Default|GetNumVectorNotSet))))
  (if (== (Variables|Default|GetNumVectorNotSet) 0)
    (for _index (range 0 (- (Variables|Default|GetNumb%20IA%20To%20Spawn) 1))
      (bind _returnvalue (Game|SpawnActorfromClass "/Game/Game/Blueprints/IA/BPChild_GameplayIA.BPChild_GameplayIA_C" (Math|Transform|MakeTransform (Math|Transform|TransformLocation (Transformation|GetActorTransform) (Utilities|Array|Get(acopy) (Variables|LocationPoint|GetSpawnLocation%20IA) _index)) (Math|Rotator|FindLookatRotation (Utilities|Array|Get(acopy) (Variables|LocationPoint|GetSpawnLocation%20IA) _index) (Variables|LocationPoint|GetGo)) "1.000000,1.000000,1.000000") "Undefined" "MultiplyWithRoot" 0 0))
      (Utilities|Array|Add (Variables|Default|GetArray%20IA%20Spawned) _returnvalue))
    (else
      ;;[0.15 0 0 0.5] Check if Spawn Location are set
      (Development|PrintString (Utilities|String|ToString(Text) (Utilities|Text|FormatText "({x}) of your IA spawn location hasn't been set" (Variables|Default|GetNumVectorNotSet))) true true "(R=1.000000,G=0.068911,B=0.000000,A=1.000000)" 2e+01))))

(event EventBeginPlay
  ;[0.15 0.15 0.15 0.5] Beginplay
  (CallFunction|SpawnIA))

(event EventOrderIA
  (params (Trigger%20TIme :type Float%20%28double-precision%29))
  (bind _returnvalue (Transformation|GetActorTransform))
  ;[0.15 0.15 0.15 0.5] Order validation
  (if (and (not (Variables|Default|GetbFinished%20Order)) (not (Variables|Default|GetbInMovement)))
    (Variables|Default|SetOrdered%20Actor (Utilities|Array|Get(acopy) (Variables|Default|GetArray%20IA%20Spawned)))
    (if (<= Trigger%20TIme 0.3)
      (if (Variables|Default|GetAuthorized%20To%20get%20Bag) :!label _label
        ;[0.15 0.15 0.15 0.5] Ia movement
        (Utilities|FlowControl|DoOnce false :!label _label_2
          (:Completed
            (Variables|Default|SetbInMovement true)
            (AI|AIMoveTo (Variables|Default|GetOrdered%20Actor) (Utilities|Select :Index (Variables|Default|GetOrderReceived) :NewEnumerator0 (Math|Transform|TransformLocation _returnvalue (Variables|LocationPoint|GetDropBag)) :NewEnumerator1 (Math|Transform|TransformLocation _returnvalue (Variables|LocationPoint|GetWait%20Gate)) :NewEnumerator2 (Math|Transform|TransformLocation _returnvalue (Variables|LocationPoint|GetGate%20Passed)) :NewEnumerator3 (Math|Transform|TransformLocation _returnvalue (Variables|LocationPoint|GetCheck%20Zone)) :NewEnumerator4 (Math|Transform|TransformLocation _returnvalue (Variables|LocationPoint|GetGet%20bag))) 0 5.0 false
              (:OnSuccess
                (Variables|Default|SetbInMovement false)
                (Utilities|FlowControl|Sequence
                  (:then_0
                    ;[0.15 0.15 0.15 0.5] Nex Order per order finished
                    (switch Utilities|FlowControl|Switch|SwitchonE_OrderPoint (Variables|Default|GetOrderReceived)
                      (:NewEnumerator0
                        (Variables|Default|SetOrderReceived "NewEnumerator1")
                        (Default|DropBelonging (Variables|Default|GetOrdered%20Actor)))
                      (:NewEnumerator1
                        (Variables|Default|SetOrderReceived "NewEnumerator2"))
                      (:NewEnumerator2
                        (if (Variables|Default|GetbCheck)
                          (Variables|Default|SetOrderReceived "NewEnumerator3")
                          (else
                            (Variables|Default|SetOrderReceived "NewEnumerator4")
                            (if (not (Variables|Default|GetBagAtEnd))
                              (Variables|Default|SetAuthorized%20To%20get%20Bag false)))))
                      (:NewEnumerator3
                        (Utilities|FlowControl|Sequence
                          (:then_0
                            (Utilities|FlowControl|DoOnce false :!label _label_3
                              (:Completed
                                (Default|RotateActor (Variables|Default|GetOrdered%20Actor)))))
                          (:then_1
                            (Variables|Default|SetOrderReceived "NewEnumerator4")
                            (if (not (Variables|Default|GetBagAtEnd))
                              (Variables|Default|SetAuthorized%20To%20get%20Bag false)))))
                      (:NewEnumerator4
                        (Variables|Default|SetbFinished%20Order true)
                        (Utilities|FlowControl|Sequence
                          (:then_0
                            (goto _label_3 Reset))
                          (:then_1
                            (Default|GetBelonging (Variables|Default|GetOrdered%20Actor))
                            (Utilities|FlowControl|Delay 1.5)
                            (AI|AIMoveTo (Variables|Default|GetOrdered%20Actor) (Math|Transform|TransformLocation (Transformation|GetActorTransform) (Variables|LocationPoint|GetGo)) 0 5.0 false
                              (:OnSuccess
                                (Transformation|Teleport (Variables|Default|GetOrdered%20Actor) (Math|Transform|TransformLocation (Transformation|GetActorTransform) (Utilities|Array|Get(acopy) (Variables|LocationPoint|GetSpawnLocation%20IA))) "0, 0, 0")
                                (Variables|Default|SetbFinished%20Order false)
                                (Variables|Default|SetbCheck false)
                                (Variables|Default|SetBagAtEnd false)
                                (Variables|Default|SetOrderReceived "NewEnumerator0")
                                (Default|ReActivate (Variables|Default|GetOrdered%20Actor)))))))))
                  (:then_1
                    (goto _label_2 Reset)))))))
        (else
          (Development|PrintString "Seems like the passenger can't get the bag")))
      (elif (>= (Variables|Default|GetOrderReceived) 2)
        (Variables|Default|SetbCheck true)
        (Variables|Default|SetOrderReceived "NewEnumerator3")
        (goto _label)
        (else
          (Development|PrintString "You did not check the passenger" true true "(R=1.000000,G=0.048921,B=0.000000,A=1.000000)" 1e+01))))))

(fn ConstructionScript
  (bind _numb_ia_to_spawn (Variables|Default|GetNumb%20IA%20To%20Spawn))
  (bind _spawnlocation_ia (Variables|LocationPoint|GetSpawnLocation%20IA))
  (bind _spawnlocation_ia_2 (Variables|LocationPoint|GetSpawnLocation%20IA))
  (bind _returnvalue (Utilities|Array|Length _spawnlocation_ia))
  ;[0.15 0.15 0.15 0.5] Create the same number of spawn location as the selected number of IA
  (for _index (range 0 (- _numb_ia_to_spawn 1))
    (if (not (== _returnvalue _numb_ia_to_spawn))
      (Utilities|Array|Add :TargetArray _spawnlocation_ia)))
  (while (> _returnvalue _numb_ia_to_spawn)
    (Utilities|Array|RemoveIndex _spawnlocation_ia_2 (Utilities|Array|LastIndex _spawnlocation_ia_2))))