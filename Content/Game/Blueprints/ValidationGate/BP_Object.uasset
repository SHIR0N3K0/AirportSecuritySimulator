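; BP_Object is a text-labeled item actor in ValidationGate that slides out and back in along a supplied spline.
; GetItemOut stores the target spline and plays a Timeline forward, while GetItemIn reverses it from the end and flags the item for destruction on finish.
; The Timeline alpha maps to distance along the spline to set world location.
; Button destroys it immediately, and the construction script sets the TextRender label.
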(event Custom|GetItemOut
  (params (Target :type Spline%20Component%20Object%20Reference))
  (Variables|Default|SetTarget Target)
  (bind _move_1 (Timeline|Timeline PlayFromStart)
    (:Update
      (Transformation|SetActorLocation (Math|Vector|MakeVector (.x (Spline|GetLocationatDistanceAlongSpline (Variables|Default|GetTarget) (Math|Float|Lerp 0.0 (Spline|GetSplineLength (Variables|Default|GetTarget)) _move_1) "World")) (.y (Spline|GetLocationatDistanceAlongSpline (Variables|Default|GetTarget) (Math|Float|Lerp 0.0 (Spline|GetSplineLength (Variables|Default|GetTarget)) _move_1) "World")) (.z (Spline|GetLocationatDistanceAlongSpline (Variables|Default|GetTarget) (Math|Float|Lerp 0.0 (Spline|GetSplineLength (Variables|Default|GetTarget)) _move_1) "World"))) false false))
    (:Finished
      (if (Variables|Default|GetItemIn)
        (Actor|DestroyActor)))))

(event Custom|GetItemIn
  (bind _target (Variables|Default|GetTarget))
  (Variables|Default|SetItemIn true)
  (bind _move_1 (Timeline|Timeline ReverseFromEnd)
    (:Update
      (Transformation|SetActorLocation (Math|Vector|MakeVector (.x (Spline|GetLocationatDistanceAlongSpline _target (Math|Float|Lerp 0.0 (Spline|GetSplineLength _target) _move_1) "World")) (.y (Spline|GetLocationatDistanceAlongSpline _target (Math|Float|Lerp 0.0 (Spline|GetSplineLength _target) _move_1) "World")) (.z (Spline|GetLocationatDistanceAlongSpline _target (Math|Float|Lerp 0.0 (Spline|GetSplineLength _target) _move_1) "World"))) false false))
    (:Finished
      (if (Variables|Default|GetItemIn)
        (Actor|DestroyActor)))))

(event EventBeginPlay)

(event Collision|EventActorBeginOverlap
  (params (OtherActor :type Actor%20Object%20Reference)))

(event EventTick
  (params (DeltaSeconds :type Float%20%28single-precision%29)))

(event EventButton
  (params (Hitted%20Component :type Primitive%20Component%20Object%20Reference))
  (Actor|DestroyActor))

(fn ConstructionScript
  (Rendering|Components|TextRender|SetText (Variables|Default|GetTextRender) (Variables|Default|GetText)))