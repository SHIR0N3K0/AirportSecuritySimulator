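; Security checkpoint gate where travellers' bags are X-rayed and inspected, and a light flashes for travellers carrying metal items.
; Dropped suitcases or bags ride timeline-driven splines to the scanner, where the green button fills the X-ray widget and red sends them on, notifying BP_IAManager.
; Clicking the bag at the end moves it for inspection and spawns its shuffled contents, including any pills or knife, along separate splines.
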(event OnComponentBeginOverlap(CheckTraveller)
  (params (OverlappedComponent :type Primitive%20Component%20Object%20Reference) (OtherActor :type Actor%20Object%20Reference) (OtherComp :type Primitive%20Component%20Object%20Reference) (OtherBodyIndex :type Integer) (bFromSweep :type Boolean) (SweepResult :type Hit%20Result%20Structure%20%28by%20ref%29))
  ;[0.15 0.15 0.15 0.5] Gate check for metalic Item
  (bind _asbpchild_gameplay_ia (Utilities|Casting|CastToBPChild_GameplayIA OtherActor))
  (if (Variables|/Game/Game/Blueprints/IA/BPChild_GameplayIA.BPChild_GameplayIA_C|GetMetalic%20Item _asbpchild_gameplay_ia)
    (Rendering|Components|Light|SetIntensity (Variables|Default|GetPointLight) 4e+04)
    (Utilities|FlowControl|Delay 2.0)
    (Rendering|Components|Light|SetIntensity (Variables|Default|GetPointLight) 0.0)))

(event Custom|MoveBelonging
  (params (Belonging :type Boolean) (Suspisious%20Item :type Boolean))
  (bind _spline (Variables|Default|GetSpline))
  (bind _bag (Variables|Default|GetBag))
  (bind _suitcase (Variables|Default|GetSuitcase))
  (bind _returnvalue (select Belonging _suitcase _bag))
  ;[0.15 0.15 0.15 0.5] Show belonging and make them move when Ai drop it's belonging
  (Variables|Default|SetbSuspisious%20Item Suspisious%20Item)
  (Variables|Default|SetbBelonging Belonging)
  (Variables|Default|SetChoosenComponent _returnvalue)
  (Rendering|SetVisibility _returnvalue true false)
  (bind _move_1 (Timeline|Move%20Spline PlayFromStart)
    (:Update
      (Transformation|SetWorldLocation (Variables|Default|GetChoosenComponent) (Math|Vector|MakeVector (.x (Spline|GetLocationatDistanceAlongSpline _spline (Math|Float|Lerp 0.0 (Spline|GetSplineLength _spline) _move_1) "World")) (.y (Spline|GetLocationatDistanceAlongSpline _spline (Math|Float|Lerp 0.0 (Spline|GetSplineLength _spline) _move_1) "World")) (.z (Transformation|GetWorldLocation (Variables|Default|GetChoosenComponent)))) false false))
    (:Finished
      (Variables|Default|SetbCan%20Push true)
      (Rendering|Components|Light|SetIntensity (Variables|Default|GetGreenLight) 5e+03))))

(event Custom|ResetCanPressGreen
  ;[0.15 0.15 0.15 0.5] Check for button pressed
  (Utilities|FlowControl|DoOnce false) ; enters at Reset
)

(event Custom|RemoveBelonging
  (bind _choosencomponent (Variables|Default|GetChoosenComponent))
  ;[0.15 0.15 0.15 0.5] Hide Belonging on threadmill when Ai pick up it's belonging
  (Rendering|SetVisibility _choosencomponent false false)
  (Transformation|SetRelativeLocation _choosencomponent (select (Variables|Default|GetbBelonging) "0, 0, 0" "0.000000,0.000000,21.000000") false false))

(event EventBeginPlay
  ;[0.15 0.15 0.15 0.5] Beginplay
  (Rendering|SetVisibility (Variables|Default|GetSuitcase) false false)
  (bind _returnvalue (Actor|GetActorOfClass "/Game/Game/Blueprints/IA/BP_IAManager.BP_IAManager_C"))
  (Variables|Default|SetIA%20Manager%20REF _returnvalue)
  (bind _aswbp_xray_sreen (Utilities|Casting|CastToWBP_XraySreen (UserInterface|GetWidget (Variables|Default|GetWidget))))
  (Variables|Default|SetAs%20WBP%20Xray%20Sreen%20REF _aswbp_xray_sreen))

(event EventTick
  (params (DeltaSeconds :type Float%20%28single-precision%29)))

(event EventButton
  (params (Hitted%20Component :type Primitive%20Component%20Object%20Reference))
  (bind _spline1 (Variables|Default|GetSpline1))
  (bind _as_wbp_xray_sreen_ref (Variables|Default|GetAs%20WBP%20Xray%20Sreen%20REF))
  (bind _objectarray (Variables|Default|GetobjectArray))
  (bind _spline2 (Variables|Default|GetSpline2))
  ;[0.15 0.15 0.15 0.5] Check for button pressed
  (if (Variables|Default|GetbCan%20Push)
    (if (== Hitted%20Component (Variables|Default|GetGreenButon))
      (Utilities|FlowControl|DoOnce false
        (:Completed
          (Default|SetScreen _as_wbp_xray_sreen_ref false (Variables|Default|GetbSuspisious%20Item))
          (Variables|Default|SetbScanned true)
          (Rendering|Components|Light|SetIntensity (Variables|Default|GetGreenLight) 0.0)
          (Rendering|Components|Light|SetIntensity (Variables|Default|GetRedLight) 5e+03)))
      (elif (== Hitted%20Component (Variables|Default|GetRedButon))
        (if (Variables|Default|GetbScanned)
          (Default|RemoveScreen _as_wbp_xray_sreen_ref)
          (Variables|Default|SetbCan%20Push false)
          (CallFunction|ResetCanPressGreen)
          (Variables|Default|SetbScanned false)
          (Rendering|Components|Light|SetIntensity (Variables|Default|GetRedLight) 0.0)
          (bind _move_1 (Timeline|Timeline PlayFromStart)
            (:Update
              (Transformation|SetWorldLocation (Variables|Default|GetChoosenComponent) (Math|Vector|MakeVector (.x (Spline|GetLocationatDistanceAlongSpline _spline1 (Math|Float|Lerp 0.0 (Spline|GetSplineLength _spline1) _move_1) "World")) (.y (Spline|GetLocationatDistanceAlongSpline _spline1 (Math|Float|Lerp 0.0 (Spline|GetSplineLength _spline1) _move_1) "World")) (.z (Transformation|GetWorldLocation (Variables|Default|GetChoosenComponent)))) false false))
            (:Finished
              (Variables|Default|SetbCanCheckBag true)
              (Variables|/Game/Game/Blueprints/IA/BP_IAManager.BP_IAManager_C|SetAuthorized%20To%20get%20Bag (Variables|Default|GetIA%20Manager%20REF) true)
              (Variables|/Game/Game/Blueprints/IA/BP_IAManager.BP_IAManager_C|SetBagAtEnd (Variables|Default|GetIA%20Manager%20REF) true))))))
    (else
      ;[0.15 0.15 0.15 0.5] Check belonging pressed
      (if (== Hitted%20Component (Variables|Default|GetChoosenComponent))
        (if (Variables|Default|GetbCanCheckBag)
          (Variables|Default|SetbCanCheckBag false)
          (bind _move_1_2 (Timeline|Timeline_0 PlayFromStart)
            (:Update
              (Transformation|SetWorldLocation (Variables|Default|GetChoosenComponent) (Math|Vector|MakeVector (.x (Spline|GetLocationatDistanceAlongSpline _spline2 (Math|Float|Lerp 0.0 (Spline|GetSplineLength _spline2) _move_1_2) "World")) (.y (Spline|GetLocationatDistanceAlongSpline _spline2 (Math|Float|Lerp 0.0 (Spline|GetSplineLength _spline2) _move_1_2) "World")) (.z (Spline|GetLocationatDistanceAlongSpline _spline2 (Math|Float|Lerp 0.0 (Spline|GetSplineLength _spline2) _move_1_2) "World"))) false false))
            (:Finished
              (Utilities|Array|Clear (Variables|Default|GetobjectArray))
              (if (Variables|Default|GetbSuspisious%20Item)
                (bind _returnvalue (Game|SpawnActorfromClass "/Game/Game/Blueprints/ValidationGate/BP_Object.BP_Object_C" (Math|Transform|MakeTransform (Transformation|GetWorldLocation (Variables|Default|GetSpline4)) "0, 0, 0" "1.000000,1.000000,1.000000") "Undefined" "MultiplyWithRoot" 0 (Utilities|Text|ToText(Name) (select (Variables|/Game/Game/Blueprints/ValidationGate/WBP_XraySreen.WBP_XraySreen_C|GetbIllegalType (Variables|Default|GetAs%20WBP%20Xray%20Sreen%20REF)) "Pills" "Knife")) 0))
                (Utilities|Array|Add (Variables|Default|GetobjectArray) _returnvalue))
              (for _array_element (Variables|/Game/Game/Blueprints/ValidationGate/WBP_XraySreen.WBP_XraySreen_C|GetUsedItems (Variables|Default|GetAs%20WBP%20Xray%20Sreen%20REF))
                (bind _returnvalue_2 (Game|SpawnActorfromClass "/Game/Game/Blueprints/ValidationGate/BP_Object.BP_Object_C" (Math|Transform|MakeTransform (Transformation|GetWorldLocation (Variables|Default|GetSpline4)) "0, 0, 0" "1.000000,1.000000,1.000000") "Undefined" "MultiplyWithRoot" 0 (Utilities|Text|ToText(Name) _array_element) 0))
                (Utilities|Array|Add (Variables|Default|GetobjectArray) _returnvalue_2))
              (Utilities|Array|Shuffle _objectarray)
              (for (_array_element_2 _array_index) _objectarray
                (Default|GetItemOut _array_element_2 (Utilities|Select :Index _array_index :Option%200 (Variables|Default|GetSpline3) :Option%201 (Variables|Default|GetSpline4) :Option%202 (Variables|Default|GetSpline5) :Option%203 (Variables|Default|GetSpline6)))))))))))

(fn ConstructionScript)