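; BPL_CeilingSpot_3m is a ceiling spot light fixture Blueprint for the airport terminal, with three spot light components.
; Its construction script applies LightIntensity to all three spots when LightOn is true, and zero otherwise.
; It also passes LightOn directly as their hidden-in-game flag, so the spots are hidden in game when switched on.
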(fn ConstructionScript
  (bind _lighton (Variables|Default|GetLightOn))
  ;[1 1 1] Base Light Logic (on/off & intensity)
  (Development|SetHiddeninGame (Variables|Default|GetSpotLight) _lighton false)
  (bind _output_get (Variables|Default|SetLightIntensity (Variables|Default|GetLightIntensity)))
  (Rendering|Components|Light|SetIntensity (Variables|Default|GetSpotLight) (select _lighton _output_get 0.0)))