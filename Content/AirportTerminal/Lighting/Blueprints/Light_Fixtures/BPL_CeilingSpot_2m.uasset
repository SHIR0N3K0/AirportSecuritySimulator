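; BPL_CeilingSpot_2m is a ceiling spot light fixture Blueprint for the airport terminal, driving two spot light components.
; Its construction script applies the LightOn flag to the visibility of both spot lights, without propagating to their children.
; It also sets both lights to the shared LightIntensity value, so the fixture's on/off state and brightness are controlled by two variables.
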(fn ConstructionScript
  (bind _lighton (Variables|Default|GetLightOn))
  ;[1 1 1] Base Light Logic (on/off & intensity)
  (Rendering|SetVisibility (Variables|Default|GetSpotLight) _lighton false)
  (Rendering|SetVisibility (Variables|Default|GetSpotLight1) _lighton false)
  (bind _output_get (Variables|Default|SetLightIntensity (Variables|Default|GetLightIntensity)))
  (Rendering|Components|Light|SetIntensity (Variables|Default|GetSpotLight) _output_get)
  (Rendering|Components|Light|SetIntensity (Variables|Default|GetSpotLight1) _output_get))